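; An actor tool that swaps one material for another across the whole level.
; The Changematerials event scans every actor's static mesh components and their material slots.
; Each slot using OriginalMaterial is set to ReplaceMaterial, and NumberMaterialChanged counts the swaps from zero on each run.
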(event Custom|Change%20materials
  (Variables|Materials|SetNumberMaterialChanged 0)
  (bind _outactors (Actor|GetAllActorsOfClass "/Script/Engine.Actor"))
  (for _array_element _outactors
    (for _array_element_2 (Actor|GetComponentsByClass _array_element "/Script/Engine.StaticMeshComponent")
      (for (_array_element_3 _array_index) (Rendering|Material|GetMaterials _array_element_2)
        (if (== _array_element_3 (Variables|Materials|GetOriginalMaterial))
          (Math|Integer|IncrementInt (Variables|Materials|GetNumberMaterialChanged)
            (:%20%20
              (Rendering|Material|SetMaterial _array_element_2 _array_index (Variables|Materials|GetReplaceMaterial)))))))))

(event EventBeginPlay)

(event Collision|EventActorBeginOverlap
  (params (OtherActor :type Actor%20Object%20Reference)))

(event EventTick
  (params (DeltaSeconds :type Float%20%28single-precision%29)))

(fn ConstructionScript)